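; BP_ClimbingCharacter is the climbing system's character Blueprint, and its graph holds only debug helpers.
; Z flip-flops global time dilation between a near freeze and normal speed, while G toggles the DrawDebug flag.
; BeginPlay and the construction script are empty, and a node chain that adds the IMC_Climbing Enhanced Input mapping context is left unconnected, so it never runs.
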(event `Key|Z`
  (params (Key :type "Key Structure"))
  (:`Pressed`
    (`/Engine/EditorBlueprintResources/StandardMacros.FlipFlop`
      (:`A`
        (`GameplayStatics.SetGlobalTimeDilation` 0.001))
      (:`B`
        (`GameplayStatics.SetGlobalTimeDilation` 1.0)))))

(event `Key|G`
  (params (Key :type "Key Structure"))
  (:`Pressed`
    (set `self.bDrawDebug` (not (`self.bDrawDebug`)))))

(event `self.ReceiveBeginPlay`)

(fn `UserConstructionScript`)